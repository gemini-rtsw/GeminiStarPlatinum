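; Player controller that switches between the controlled pawn's free view and four fixed BP_ViewCamera views.
; On BeginPlay it adds the input mapping, indexes cameras by SortIndex, and creates a camera indicator widget inside that loop, once per camera.
; Direct-select and cycle inputs call SetViewIndex, which wraps the index, blends the view target and blocks look/move input on fixed views.
; An OnViewChanged dispatcher passes view name and hint to the indicator.
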(event `self.ReceiveBeginPlay`
  (`EnhancedInputSubsystemInterface.AddMappingContext` (subsystem `EnhancedInputLocalPlayerSubsystem`) "/Game/Input/IMC_CameraViews.IMC_CameraViews" 0 (struct))
  (bind _outactors (`GameplayStatics.GetAllActorsOfClass` "/Game/Blueprints/BP_ViewCamera.BP_ViewCamera_C"))
  (for _array_element _outactors
    (`BlueprintMapLibrary.Map_Add` (`self.ViewCameras`) (`/Game/Blueprints/BP_ViewCamera.SortIndex` _array_element) _array_element)
    (`WidgetBlueprintLibrary.SetInputMode_GameAndUIEx` (`GameplayStatics.GetPlayerController` 0) null)
    (bind _returnvalue (`|CreateWidget` "/Game/Blueprints/WB_CameraIndicator.WB_CameraIndicator_C"))
    (`UserWidget.AddToViewport` _returnvalue 0)
    (set `self.CameraIndicator` _returnvalue)))

(event `OnViewChanged_Event`
  (params (ViewName :type String) (HintText :type String))
  (`/Game/Blueprints/WB_CameraIndicator.OnViewChanged_Event` (`self.CameraIndicator`) ViewName HintText))

(event `EnhancedInput|/Game/Input/IA_CycleView`
  (params (ActionValue :type Boolean) (ElapsedSeconds :type "Float (double-precision)") (TriggeredSeconds :type "Float (double-precision)") (InputAction :type "InputAction Object Reference" :default "/Game/Input/IA_CycleView.IA_CycleView"))
  (:`Triggered`
    (`self.SetViewIndex` (+ (`self.CurrentViewIndex`) 1))))

(event `EnhancedInput|/Game/Input/IA_View0`
  (params (ActionValue :type Boolean) (ElapsedSeconds :type "Float (double-precision)") (TriggeredSeconds :type "Float (double-precision)") (InputAction :type "InputAction Object Reference" :default "/Game/Input/IA_View0.IA_View0"))
  (:`Triggered`
    (`self.SetViewIndex` 0)))

(event `EnhancedInput|/Game/Input/IA_View1`
  (params (ActionValue :type Boolean) (ElapsedSeconds :type "Float (double-precision)") (TriggeredSeconds :type "Float (double-precision)") (InputAction :type "InputAction Object Reference" :default "/Game/Input/IA_View1.IA_View1"))
  (:`Triggered`
    (`self.SetViewIndex` 1)))

(event `EnhancedInput|/Game/Input/IA_View2`
  (params (ActionValue :type Boolean) (ElapsedSeconds :type "Float (double-precision)") (TriggeredSeconds :type "Float (double-precision)") (InputAction :type "InputAction Object Reference" :default "/Game/Input/IA_View2.IA_View2"))
  (:`Triggered`
    (`self.SetViewIndex` 2)))

(event `EnhancedInput|/Game/Input/IA_View4`
  (params (ActionValue :type Boolean) (ElapsedSeconds :type "Float (double-precision)") (TriggeredSeconds :type "Float (double-precision)") (InputAction :type "InputAction Object Reference" :default "/Game/Input/IA_View4.IA_View4"))
  (:`Triggered`
    (`self.SetViewIndex` 4)))

(event `EnhancedInput|/Game/Input/IA_View3`
  (params (ActionValue :type Boolean) (ElapsedSeconds :type "Float (double-precision)") (TriggeredSeconds :type "Float (double-precision)") (InputAction :type "InputAction Object Reference" :default "/Game/Input/IA_View3.IA_View3"))
  (:`Triggered`
    (`self.SetViewIndex` 3)))

(fn `SetViewIndex`
  (params (NewIndex :type Integer))
  (bind _returnvalue (`self.WrapInteger` NewIndex 0 4))
  (if (== _returnvalue 0)
    (`self.SetViewTargetWithBlend` (`self.K2_GetPawn`) 0.0 "VTBlend_Linear" 0.22)
    (`self.ResetIgnoreLookInput`)
    (`self.ResetIgnoreMoveInput`)
    (set `self.CurrentViewIndex` _returnvalue)
    (`self.OnViewChanged` "Free" "C")
    (else
      (`self.SetViewTargetWithBlend` (`BlueprintMapLibrary.Map_Find` (`self.ViewCameras`) _returnvalue) 0.0 "VTBlend_Linear" 0.22)
      (`self.SetIgnoreLookInput` true)
      (`self.SetIgnoreMoveInput` true)
      (bind _output_get (set `self.CurrentViewIndex` _returnvalue))
      (`self.OnViewChanged` (`KismetTextLibrary.Conv_TextToString` (`/Game/Blueprints/BP_ViewCamera.DisplayName` (`BlueprintMapLibrary.Map_Find` (`self.ViewCameras`) _output_get))) "C"))))

(fn `UserConstructionScript`
  (add `self.OnViewChanged` (`|CreateDelegate` :!event `OnViewChanged_Event`)))

(fn `WrapInteger`
  (params (Number :type Integer) (Min :type Integer) (Max :type Integer))
  (returns (ReturnValue :type Integer))
  (bind _returnvalue (mod (- Number Min) (- Max Min -1)))
  (if (< _returnvalue 0)
    (return (+ (`local.Max`) _returnvalue 1))
    (else
      (return (+ _returnvalue Min)))))