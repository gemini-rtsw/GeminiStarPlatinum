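; BP_EnvironmentViewNew drives a CelestialVault sky from a time-changed event, keeping the vault's date and time of day in step with the given time.
; When the day, month or year differs, it copies the new date into the vault and rebuilds it.
; It then sets the time of day in fractional hours and plays or pauses the vault depending on whether time progresses.
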(event `self.OnTimeChanged`
  (params (NewTime :type "DateTime Structure") (TimeProgresses :type Boolean))
  (bind _returnvalue (`KismetMathLibrary.GetYear` NewTime))
  (bind _returnvalue_2 (`KismetMathLibrary.GetMonth` NewTime))
  (bind _returnvalue_3 (`KismetMathLibrary.GetDay` NewTime))
  (bind _celestialvault (`self.CelestialVault`))
  (bind _celestialvault_2 (`self.CelestialVault`))
  (if (`KismetSystemLibrary.IsValid` _celestialvault)
    (if (or (!= _returnvalue_3 (`CelestialVaultDaySequenceActor.Day` _celestialvault)) (!= _returnvalue_2 (`CelestialVaultDaySequenceActor.Month` _celestialvault)) (!= _returnvalue (`CelestialVaultDaySequenceActor.Year` _celestialvault)))
      (set `CelestialVaultDaySequenceActor.Year` _returnvalue _celestialvault_2)
      (set `CelestialVaultDaySequenceActor.Month` _returnvalue_2 _celestialvault_2)
      (set `CelestialVaultDaySequenceActor.Day` _returnvalue_3 _celestialvault_2)
      (`CelestialVaultDaySequenceActor.RebuildAll` _celestialvault_2))
    (`DaySequenceActor.SetTimeOfDay` _celestialvault_2 (`KismetMathLibrary.Conv_IntToDouble` (+ (`KismetMathLibrary.GetHour` NewTime) (/ (`KismetMathLibrary.GetMinute` NewTime) 60) (/ (`KismetMathLibrary.GetSecond` NewTime) 3600))))
    (if TimeProgresses
      (`DaySequenceActor.Play` _celestialvault_2)
      (else
        (`DaySequenceActor.Pause` _celestialvault_2)))))

(fn `UserConstructionScript`)